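; VR plate actor that can be picked up until it is washed, and dropped off.
; On BeginPlay it plays a sound at the plate and binds its removal event to MyVRGameMode, which destroys the actor when triggered.
; PickUp disables physics and attaches the root to the grabbing component, keeping world transform.
; DropOff re-enables physics and detaches the actor.
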(event Custom|RemovePlateEvent
  ;[1 1 1] Event to remove plate from game
  (Actor|DestroyActor))

(event EventBeginPlay
  ;[1 1 1] Prepare plate to remove
  (Audio|PlaySoundatLocation 0 (Transformation|GetWorldLocation (Variables|Default|Getplate)))
  (bind _asmy_vrgame_mode (Utilities|Casting|CastToMyVRGameMode (Game|GetGameMode)))
  (bind _output_get (Variables|Default|SetmyVRGameMode _asmy_vrgame_mode))
  (EventDispatchers|BindEventtoRemovePlates _output_get (delegate Custom|RemovePlateEvent)))

(event Collision|EventActorBeginOverlap
  (params (OtherActor :type Actor%20Object%20Reference)))

(event EventTick
  (params (DeltaSeconds :type Float%20%28single-precision%29)))

(event EventDropOff
  ;[1 1 1] Drop off plate
  (Physics|SetSimulatePhysics (Variables|Default|Getplate) true)
  (Transformation|DetachFromActor "KeepWorld" "KeepWorld" "KeepWorld"))

(event EventPickUp
  (params (ActorToAttachTo :type Scene%20Component%20Object%20Reference))
  ;[1 1 1] Pick up plate
  (if (not (Variables|Default|GetisWashed))
    (Physics|SetSimulatePhysics (Variables|Default|Getplate) false)
    (Transformation|AttachComponentToComponent (VehicleSound|GetRootComponent) ActorToAttachTo "None" "KeepWorld" "KeepWorld" "KeepWorld" true)))

(fn ConstructionScript)