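; Sink actor that washes plates and awards score in a VR game.
; On overlap with an unwashed bp_plate, it marks the plate washed, plays a splash sound at the SinkBox and sets a short lifespan so the plate despawns.
; It then tells MyVRGameMode to increase the score, with the IsWashed flag preventing repeat scoring.
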(event EventBeginPlay)

(event Collision|EventActorBeginOverlap
  (params (OtherActor :type Actor%20Object%20Reference))
  ;[1 1 1] Wash plate and increase score
  (Utilities|IsValid OtherActor
    (:Is%20Valid
      (bind _asbp_plate (Utilities|Casting|CastTobp_plate OtherActor))
      (if (not (Variables|/Game/Assets/blueprints/bp_plate.bp_plate_C|GetisWashed _asbp_plate))
        (Variables|/Game/Assets/blueprints/bp_plate.bp_plate_C|SetisWashed _asbp_plate true)
        (Audio|PlaySoundatLocation "/Game/Assets/audio/water-splash_Cue.water-splash_Cue" (Transformation|GetWorldLocation (Variables|Default|GetSinkBox)))
        (Actor|SetLifeSpan _asbp_plate 2.0)
        (bind _asmy_vrgame_mode (Utilities|Casting|CastToMyVRGameMode (Game|GetGameMode)))
        (Default|IncreaseScore _asmy_vrgame_mode)))))

(event EventTick
  (params (DeltaSeconds :type Float%20%28single-precision%29)))

(fn ConstructionScript)